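; BP_Rocket is a collection rocket that launches once the player's BP_PhysicsBall has at most one entry left in ItemsToGet.
; Actors overlapping the InsideBin component are removed from that list if present.
; Tick polls the list length and calls BlastOff every frame the condition holds.
; BlastOff applies a continuous upward force to the Can component as a mass-independent acceleration.
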(event `self.ReceiveTick`
  (params (DeltaSeconds :type "Float (single-precision)"))
  (bind _asbp_physics_ball (cast `/Game/MyContent/BP/BP_PhysicsBall` (`GameplayStatics.GetPlayerPawn` 0)))
  (if (<= (`KismetArrayLibrary.Array_Length` (`/Game/MyContent/BP/BP_PhysicsBall.ItemsToGet` _asbp_physics_ball)) 1)
    (`self.BlastOff`)))

(event `self.InsideBin.OnComponentBeginOverlap`
  (params (OverlappedComponent :type "PrimitiveComponent Object Reference") (OtherActor :type "Actor Object Reference") (OtherComp :type "PrimitiveComponent Object Reference") (OtherBodyIndex :type Integer) (bFromSweep :type Boolean) (SweepResult :type "HitResult Structure (by ref)"))
  (bind _asbp_physics_ball (cast `/Game/MyContent/BP/BP_PhysicsBall` (`GameplayStatics.GetPlayerPawn` 0)))
  (bind _returnvalue (`KismetArrayLibrary.Array_Find` (`/Game/MyContent/BP/BP_PhysicsBall.ItemsToGet` _asbp_physics_ball) OtherActor))
  (if (!= _returnvalue -1)
    (`KismetArrayLibrary.Array_Remove` (`/Game/MyContent/BP/BP_PhysicsBall.ItemsToGet` _asbp_physics_ball) _returnvalue)))

(fn `BlastOff`
  (`PrimitiveComponent.AddForce` (`self.Can`) (0.0 0.0 10000.0) "None" true))

(fn `UserConstructionScript`)